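; BP_NormalTree is a tree actor with Stem and Leaf meshes that adjusts its rendering once gameplay starts.
; BeginPlay caches the BP_NEOGameState, and Tick polls it until the state is OnGamePlaying.
; It then clears any forced LOD on both meshes (0 means automatic), applies a distance cull to each, and disables its own tick so the setup runs once.
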(event EventBeginPlay
  (bind _asbp_neogame_state (Utilities|Casting|CastToBP_NEOGameState (Game|GetGameState)))
  (Variables|Default|SetAs%20BP%20NEOGame%20State _asbp_neogame_state))

(event Collision|EventActorBeginOverlap
  (params (OtherActor :type Actor%20Object%20Reference)))

(event EventTick
  (params (DeltaSeconds :type Float%20%28single-precision%29))
  (if (Utilities|Enum|Equal(Enum) (Class|NEOGameState|GetGameState (Variables|Default|GetAs%20BP%20NEOGame%20State)) "OnGamePlaying")
    (Rendering|LOD|SetForcedLodModel (Variables|Default|Getstem) 0)
    (Rendering|LOD|SetForcedLodModel (Variables|Default|GetLeaf) 0)
    (Class|PrimitiveComponent|SetCullDistance (Variables|Default|Getstem) 4e+03)
    (Class|PrimitiveComponent|SetCullDistance (Variables|Default|GetLeaf) 4e+03)
    (Actor|Tick|SetActorTickEnabled false)))

(fn ConstructionScript)