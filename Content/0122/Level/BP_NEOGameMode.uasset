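; BP_NEOGameMode is a Game Mode that shows a screen fade overlay during battle transitions.
; On BeginPlay it creates a BP_Black widget and stores it as Smoke.
; BattleStartEvent adds the widget to the viewport and plays its fade-in, while BattleFinishEvent plays the fade-out and removes it once the animation finishes.
; DestroyerEvent is declared but empty.
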(event Custom|BattleStartEvent
  (bind _smoke (Variables|Default|GetSmoke))
  (UserInterface|Viewport|AddtoViewport _smoke 0)
  (Components|Animation|PlayAnimation _smoke (Variables|/Game/0122/Level/BP_Black.BP_Black_C|GetFadein _smoke) 0.0))

(event Custom|BattleFinishEvent
  (bind _smoke (Variables|Default|GetSmoke))
  (Components|Animation|PlayAnimation _smoke (Variables|/Game/0122/Level/BP_Black.BP_Black_C|GetFadeOut _smoke) 0.0
    (:Finished
      (Widget|RemovefromParent _smoke))))

(event EventBeginPlay
  (bind _returnvalue (UserInterface|CreateWidget "/Game/0122/Level/BP_Black.BP_Black_C"))
  (Variables|Default|SetSmoke _returnvalue))

(event EventDestroyerEvent)

(fn ConstructionScript)