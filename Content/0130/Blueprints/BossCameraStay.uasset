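; BossCameraStay is an overlap trigger for a boss encounter's camera.
; The first overlap by an actor tagged Player finds BP_SplineCamera and calls AirWallSwitch(true), guarded by DoOnce.
; An unconnected chain, which never runs, would play BossStartMovie with BP_OdaNobunaga bound as Boss, create the boss widget, and call AirWallSwitch(false).
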(event Custom|CustomEvent)

(event EventBeginPlay
  (|CallParentFunction) ; このノードは無効になっているため呼び出せません。\n機能をビルドするにはピンをドラッグしてください。
)

(event Collision|EventActorBeginOverlap
  (params (OtherActor :type Actor%20Object%20Reference))
  (if (Actor|ActorHasTag OtherActor "Player")
    (Utilities|FlowControl|DoOnce false
      (:Completed
        (bind _returnvalue (Actor|GetActorOfClass "/Game/0130/Blueprints/BP_SplineCamera.BP_SplineCamera_C"))
        (Default|AirWallSwitch _returnvalue true)))))

(event EventTick
  (params (DeltaSeconds :type Float%20%28single-precision%29))
  (|CallParentFunction DeltaSeconds) ; このノードは無効になっているため呼び出せません。\n機能をビルドするにはピンをドラッグしてください。
)

(fn ConstructionScript
  (|CallParentFunction))